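; MyGameMode is a game mode that spawns and possesses a Sedan for each player who logs in, in what appears to be a lap-based racing game.
; PostLogin stores each MyPlayerController and places its car at the PlayerStart looked up by the player's zero-based join index as name.
; InitCheckpoints collects all Checkpoint actors and InitSettings copies max laps from the level's Tracker; neither is called within this Blueprint.
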(event `self.K2_PostLogin`
  (params (NewPlayer :type "PlayerController Object Reference"))
  ;[1 1 1] Spawning Players on PlayerStart locations of the map. (This prevents such behavior like start game inside textures at the beginning)
  (bind _asmy_player_controller (cast `/Game/Blueprints/MyPlayerController` NewPlayer))
  (bind _output_get (set `self.PlayerControllerRef` _asmy_player_controller))
  (`KismetArrayLibrary.Array_Add` (`self.GM_Players`) _output_get)
  (bind _returnvalue (`|SpawnActorFromClass` "/Game/MAP/Vehicle/Sedan/Sedan.Sedan_C" (`self.GetTransform` (`self.K2_FindPlayerStart` NewPlayer (`KismetStringLibrary.Conv_IntToString` (- (`KismetArrayLibrary.Array_Length` (`self.GM_Players`)) 1)))) "Undefined" "OverrideRootScale" null null))
  (`Controller.Possess` (`self.PlayerControllerRef`) _returnvalue)
  (`KismetSystemLibrary.PrintString` "Hello"))

(fn `InitCheckpoints`
  (bind _outactors (`GameplayStatics.GetAllActorsOfClass` "/Game/Blueprints/Checkpoint.Checkpoint_C"))
  (for _array_element _outactors
    (`KismetArrayLibrary.Array_Add` (`self.GM_Checkpoints`) _array_element)))

(fn `InitSettings`
  (bind _returnvalue (`GameplayStatics.GetActorOfClass` "/Game/Blueprints/Tracker.Tracker_C"))
  (set `self.GM_MaxLaps` (`/Game/Blueprints/Tracker.MaxLaps` _returnvalue)))

(fn `UserConstructionScript`)