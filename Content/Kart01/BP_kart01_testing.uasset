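; BP_kart01_testing is a test kart Blueprint driven by keyboard and mouse through a VehicleMovement component.
; Hardcoded W/S and A/D key events set full throttle, reverse throttle and steering, zeroing them on release, while Space holds the handbrake.
; MouseX and MouseY axis events add relative yaw and pitch to the SpringArm without clamping.
; An unconnected console command for PhysX collision visualization never runs.
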(event `InputAxisKey|MouseX`
  (params (AxisValue :type "Float (single-precision)"))
  (`SceneComponent.K2_AddRelativeRotation` (`self.SpringArm`) (`KismetMathLibrary.MakeRotator` 0.0 0.0 AxisValue) false false))

(event `InputAxisKey|MouseY`
  (params (AxisValue :type "Float (single-precision)"))
  (`SceneComponent.K2_AddRelativeRotation` (`self.SpringArm`) (`KismetMathLibrary.MakeRotator` 0.0 AxisValue) false false))

(event `Key|SpaceBar`
  (params (Key :type "Key Structure"))
  (bind _vehiclemovement (`self.VehicleMovement`))
  (:`Pressed`
    (`WheeledVehicleMovementComponent.SetHandbrakeInput` _vehiclemovement true))
  (:`Released`
    (`WheeledVehicleMovementComponent.SetHandbrakeInput` _vehiclemovement false)))

(event `self.ReceiveBeginPlay`)

(event `Key|W`
  (params (Key :type "Key Structure"))
  (bind _vehiclemovement (`self.VehicleMovement`))
  (:`Pressed`
    (`WheeledVehicleMovementComponent.SetThrottleInput` _vehiclemovement 1.0))
  (:`Released`
    (`WheeledVehicleMovementComponent.SetThrottleInput` _vehiclemovement 0.0 :!label _label)))

(event `Key|S`
  (params (Key :type "Key Structure"))
  (:`Pressed`
    (`WheeledVehicleMovementComponent.SetThrottleInput` (`self.VehicleMovement`) -1.0))
  (:`Released`
    (goto _label)))

(event `Key|A`
  (params (Key :type "Key Structure"))
  (bind _vehiclemovement (`self.VehicleMovement`))
  (:`Pressed`
    (`WheeledVehicleMovementComponent.SetSteeringInput` _vehiclemovement -1.0))
  (:`Released`
    (`WheeledVehicleMovementComponent.SetSteeringInput` _vehiclemovement 0.0 :!label _label_2)))

(event `Key|D`
  (params (Key :type "Key Structure"))
  (:`Pressed`
    (`WheeledVehicleMovementComponent.SetSteeringInput` (`self.VehicleMovement`) 1.0))
  (:`Released`
    (goto _label_2)))

(fn `UserConstructionScript`)