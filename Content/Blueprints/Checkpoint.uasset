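; Kart racing checkpoint that records a player's progress and respawn point on their PlayerState when a kart leaves its trigger.
; On end overlap, it accepts either BP_kart or BP_kart2 and dots the kart's velocity with the Arrow's forward vector, counting only forward passes.
; A valid pass sends the checkpoint number and the checkpoint's location, without its rotation, to SetPassedCheckpointsArray on PS_MyPlayerState.
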(event `self.Trigger.OnComponentEndOverlap`
  (params (OverlappedComponent :type "PrimitiveComponent Object Reference") (OtherActor :type "Actor Object Reference") (OtherComp :type "PrimitiveComponent Object Reference") (OtherBodyIndex :type Integer))
  ;[1 1 1] Checkpoint System - Cleared when Overlapping Ends then set Player's respawn location
  (bind _asbp_kart (cast `/Game/Kart01/BP_kart` OtherActor)
    (:`then`
      (bind _asps_my_player_state (cast `/Game/Blueprints/PS_MyPlayerState` (`Pawn.PlayerState` _asbp_kart)))
      (if (> (`KismetMathLibrary.Dot_VectorVector` (`self.GetVelocity` _asbp_kart) (`KismetMathLibrary.Conv_RotatorToVector` (`SceneComponent.K2_GetComponentRotation` (`self.Arrow`)))) 0.0)
        (`/Game/Blueprints/PS_MyPlayerState.SetPassedCheckpointsArray` _asps_my_player_state (`self.CheckpointNumber`) (`KismetMathLibrary.Conv_VectorToTransform` (`self.K2_GetActorLocation`)))))
    (:`CastFailed`
      (bind _asbp_kart_2 (cast `/Game/Kart02/BP_kart2` OtherActor))
      (bind _asps_my_player_state_2 (cast `/Game/Blueprints/PS_MyPlayerState` (`Pawn.PlayerState` _asbp_kart_2)))
      (if (> (`KismetMathLibrary.Dot_VectorVector` (`self.GetVelocity` _asbp_kart_2) (`KismetMathLibrary.Conv_RotatorToVector` (`SceneComponent.K2_GetComponentRotation` (`self.Arrow`)))) 0.0)
        (`/Game/Blueprints/PS_MyPlayerState.SetPassedCheckpointsArray` _asps_my_player_state_2 (`self.CheckpointNumber`) (`KismetMathLibrary.Conv_VectorToTransform` (`self.K2_GetActorLocation`)))))))

(fn `UserConstructionScript`)